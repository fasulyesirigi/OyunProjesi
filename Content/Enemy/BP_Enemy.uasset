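; BP_Enemy is a melee enemy character that detects the player, attacks with a sword, takes damage and dies.
; Pawn sensing sets blackboard keys and run speed; AttackPlayer sphere-traces ahead and plays a random attack montage.
; A looping timer line-traces between sword sockets, damaging the player unless blocking.
; Damage updates a health bar widget, shown on trigger overlap; death flags the blackboard, removes the capsule and destroys the actor after a delay.
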(event `Reference`
  ;[1 1 1] References
  (bind _asbp_character (cast `/Game/FPSwordAndShield/Blueprints/BP_Character` (`GameplayStatics.GetPlayerCharacter` 0)))
  (set `self.CharacterRef` _asbp_character)
  (bind _asw_ai_health_bar (cast `/Game/UI/W_AI_HealthBar` (`WidgetComponent.GetUserWidgetObject` (`self.HealthBar`))))
  (bind _output_get (set `self.HealthBarRef` _asw_ai_health_bar))
  (set `/Game/UI/W_AI_HealthBar.Health` (`self.Health`) _output_get))

(event `TriggerSword`
  ;[1 1 1] Sword Trace
  (bind _returnvalue (`KismetSystemLibrary.K2_SetTimerDelegate` (delegate `SwordLineTrace`) 0.05 true))
  (set `self.Trigger Sword Event` _returnvalue))

(event `StopTriggerSword`
  ;[1 1 1] Sword Trace
  (`KismetSystemLibrary.K2_ClearAndInvalidateTimerHandle` (`self.Trigger Sword Event`)))

(event `SwordLineTrace`
  (bind _mesh (`self.Mesh`))
  ;[1 1 1] Sword Trace
  (bind _outhit (`KismetSystemLibrary.LineTraceSingleForObjects` :`Start` (`SceneComponent.GetSocketLocation` _mesh "Start") :`End` (`SceneComponent.GetSocketLocation` _mesh "End") :`ObjectTypes` (`|MakeArray` "ObjectTypeQuery3" :!type "EObjectTypeQuery Enum") :`DrawDebugType` "ForDuration"))
  (bind (_bblockinghit _binitialoverlap _time _distance _location _impactpoint _normal _impactnormal _physmat _hitactor) (`GameplayStatics.BreakHitResult` _outhit))
  (bind _asbp_character (cast `/Game/FPSwordAndShield/Blueprints/BP_Character` _hitactor))
  (if (not (`/Game/FPSwordAndShield/Blueprints/BP_Character.Blocking?` _asbp_character))
    (`GameplayStatics.ApplyDamage` _hitactor 10.0)))

(event `self.ReceiveBeginPlay`
  ;[1 1 1] Begin Play
  (`BlackboardComponent.SetValueAsBool` (`AIBlueprintHelperLibrary.GetBlackboard` (`AIBlueprintHelperLibrary.GetAIController` self)) "IsDead?" false)
  (`self.Reference`))

(event `self.PawnSensing.OnSeePawn`
  (params (Pawn :type "Pawn Object Reference"))
  ;[1 1 1] Character Seen
  (if (not (`self.Is Dead`))
    (cast `/Game/FPSwordAndShield/Blueprints/BP_Character` Pawn)
    (`BlackboardComponent.SetValueAsBool` (`AIBlueprintHelperLibrary.GetBlackboard` (`AIBlueprintHelperLibrary.GetAIController` self)) "CharacterSeen?" true)
    (set `CharacterMovementComponent.MaxWalkSpeed` (`self.RunSpeed`) (`self.CharacterMovement`))
    (`KismetSystemLibrary.PrintString` "Karakter görüldü")))

(event `AttackPlayer`
  (bind _returnvalue (`self.K2_GetActorLocation`))
  ;[1 1 1] Attack
  (bind (_outhit _returnvalue_2) (`KismetSystemLibrary.SphereTraceSingleForObjects` :`Start` _returnvalue :`End` (+ _returnvalue (* (`KismetMathLibrary.GetForwardVector` (`self.K2_GetActorRotation`)) 250.0)) :`Radius` 150.0 :`ObjectTypes` (`|MakeArray` "ObjectTypeQuery3" :!type "EObjectTypeQuery Enum") :`DrawDebugType` "ForDuration"))
  (if _returnvalue_2
    (`self.PlayAnimMontage` (`KismetArrayLibrary.Array_Random` (`self.Anim Montage`)))))

(event `self.ReceiveAnyDamage`
  (params (Damage :type "Float (single-precision)") (DamageType :type "DamageType Object Reference") (InstigatedBy :type "Controller Object Reference") (DamageCauser :type "Actor Object Reference"))
  ;[1 1 1] Any Damage
  (`/Engine/EditorBlueprintResources/StandardMacros.DoOnce` false :!label _label
    (:`Completed`
      (bind _output_get (set `self.Health` (- (`self.Health`) Damage)))
      (set `/Game/UI/W_AI_HealthBar.Health` _output_get (`self.HealthBarRef`))
      (if (<= _output_get 0.0)
        (`BlackboardComponent.SetValueAsBool` (`AIBlueprintHelperLibrary.GetBlackboard` (`AIBlueprintHelperLibrary.GetAIController` self)) "IsDead?" true)
        (set `self.Is Dead` true)
        (`ActorComponent.K2_DestroyComponent` (`self.CapsuleComponent`))
        (`KismetSystemLibrary.Delay` 6.0)
        (`self.K2_DestroyActor` self)
        (else
          (goto _label :!via `Reset`))))))

(event `self.Trigger.OnComponentBeginOverlap`
  (params (OverlappedComponent :type "PrimitiveComponent Object Reference") (OtherActor :type "Actor Object Reference") (OtherComp :type "PrimitiveComponent Object Reference") (OtherBodyIndex :type Integer) (bFromSweep :type Boolean) (SweepResult :type "HitResult Structure (by ref)"))
  ;[1 1 1] Health Bar Visibility
  (`SceneComponent.SetVisibility` (`self.HealthBar`) true false))

(event `self.Trigger.OnComponentEndOverlap`
  (params (OverlappedComponent :type "PrimitiveComponent Object Reference") (OtherActor :type "Actor Object Reference") (OtherComp :type "PrimitiveComponent Object Reference") (OtherBodyIndex :type Integer))
  ;[1 1 1] Health Bar Visibility
  (`SceneComponent.SetVisibility` (`self.HealthBar`) false false))

(fn `UserConstructionScript`)