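; BP_EnemySpawner is an actor that spawns growing waves of BP_Enemy at its own transform.
; On BeginPlay it binds SpawnEnemy to the RespawnEnemy event on FirstPersonGameMode.
; Each call spawns EnemySpawned enemies, adjusting for collisions, then raises that count by an ever-larger increment.
; Spawning stops once the count reaches a fixed cap.
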(event `self.ReceiveBeginPlay`
  (bind _asfirst_person_game_mode (cast `/Game/FPSwordAndShield/Blueprints/FirstPersonGameMode` (`GameplayStatics.GetGameMode`)))
  (bind _output_get (set `self.GameMode` _asfirst_person_game_mode))
  (add `/Game/FPSwordAndShield/Blueprints/FirstPersonGameMode.RespawnEnemy` _output_get (delegate `Spawn Enemy`)))

(event `Spawn Enemy`
  (bind _enemy_increment (`self.Enemy Increment`))
  (if (< (`self.Enemy Spawned`) 8)
    (for _ (range (`self.Enemy Spawned`))
      (`|SpawnActorFromClass` "/Game/Enemy/BP_Enemy.BP_Enemy_C" (`self.GetTransform`) "AdjustIfPossibleButAlwaysSpawn" "OverrideRootScale" null null))
    (`/Engine/EditorBlueprintResources/StandardMacros.IncrementInt` _enemy_increment
      (:`  `
        (set `self.Enemy Spawned` (+ _enemy_increment (`self.Enemy Spawned`)))))))

(fn `UserConstructionScript`)